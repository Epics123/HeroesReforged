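; Base actor for spline rails that the player rides, with homing targets at the ends and switching to neighboring rails.
; Construction script builds collidable spline meshes along RailSpline and, on open rails, adds an inset homing target at each end.
; Reaching a target sets both targets' launch velocity along player forward.
; While PlayerRef is valid, Tick sphere-traces sideways by lean direction to set the player's JumpRail, with console-variable debug drawing.
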(event `self.ReceiveBeginPlay`
  (if (and (`KismetSystemLibrary.IsValid` (`self.StartHomingTarget`)) (`KismetSystemLibrary.IsValid` (`self.EndHomingTarget`)))
    (add `/Game/LevelObjects/BP_HomingTarget_Base.OnHomingTargetReached` (`self.StartHomingTarget`) (`|CreateDelegate` :!event `HomingTargetReached`))
    (add `/Game/LevelObjects/BP_HomingTarget_Base.OnHomingTargetReached` (`self.EndHomingTarget`) (`|CreateDelegate` :!event `HomingTargetReached`))
    (set `HomingTargetComponent.DeflectionStrength` 0.0 (`/Game/LevelObjects/BP_HomingTarget_Base.BPC_HomingTarget` (`self.StartHomingTarget`)))
    (set `HomingTargetComponent.DeflectionStrength` 0.0 (`/Game/LevelObjects/BP_HomingTarget_Base.BPC_HomingTarget` (`self.EndHomingTarget`)))))

(event `self.ReceiveTick`
  (params (DeltaSeconds :type "Float (single-precision)"))
  (bind _returnvalue (`SplineComponent.GetLocationAtDistanceAlongSpline` (`self.RailSpline`) (`SplineComponent.GetDistanceAlongSplineAtLocation` (`self.RailSpline`) (`self.K2_GetActorLocation` (`self.PlayerRef`)) "World") "World"))
  (`/Engine/EditorBlueprintResources/StandardMacros.IsValid` (`self.PlayerRef`)
    (:`Is Valid`
      (bind _returnvalue_2 (`KismetSystemLibrary.GetConsoleVariableIntValue` "Gameplay.Debug.Rails"))
      (bind (_outhit _returnvalue_3) (`KismetSystemLibrary.SphereTraceSingleForObjects` :`Start` _returnvalue :`End` (+ _returnvalue (* (* (`self.GetActorRightVector` (`self.PlayerRef`)) (`KismetMathLibrary.Round` (`HeroCharacter.RailLeanDirection` (`self.PlayerRef`)))) (`self.RailSwitchTraceDistance`))) :`Radius` 10.0 :`ObjectTypes` (`|MakeArray` "ObjectTypeQuery8" :!type "EObjectTypeQuery Enum") :`DrawDebugType` (select `bool` (!= _returnvalue_2 0) :`true` "ForOneFrame" :!type "EDrawDebugTrace Enum")))
      (if _returnvalue_3
        (bind _asbp_rail_base (cast `/Game/LevelObjects/Rails/BP_RailBase` (`.HitActor` (`GameplayStatics.BreakHitResult` _outhit))))
        (set `HeroCharacter.JumpRail` _asbp_rail_base (`self.PlayerRef`))
        (else
          (set `HeroCharacter.JumpRail` null (`self.PlayerRef`)))))))

(event `HomingTargetReached`
  (set `HomingTargetComponent.LaunchVelocity` (* (`self.GetActorForwardVector` (`GameplayStatics.GetPlayerCharacter` 0)) (`self.RailHomingVelocity`)) (`/Game/LevelObjects/BP_HomingTarget_Base.BPC_HomingTarget` (`self.StartHomingTarget`)))
  (set `HomingTargetComponent.LaunchVelocity` (* (`self.GetActorForwardVector` (`GameplayStatics.GetPlayerCharacter` 0)) (`self.RailHomingVelocity`)) (`/Game/LevelObjects/BP_HomingTarget_Base.BPC_HomingTarget` (`self.EndHomingTarget`))))

(fn `UserConstructionScript`
  (bind _railspline (`self.RailSpline`))
  (bind _railspline_2 (`self.RailSpline`))
  (bind _returnvalue (- (`SplineComponent.GetNumberOfSplinePoints` _railspline_2) 1))
  (`parent.UserConstructionScript`)
  (`KismetArrayLibrary.Array_Clear` (`self.RailMeshComponents`))
  (for _index (range (+ (- (`SplineComponent.GetNumberOfSplinePoints` (`self.RailSpline`)) (`KismetMathLibrary.SelectInt` 1 2 (`SplineComponent.IsClosedLoop` (`self.RailSpline`)))) 1))
    (bind _returnvalue_2 (`AddComponent|NODE_AddSplineMeshComponent-0`))
    (`SceneComponent.K2_AttachToComponent` _returnvalue_2 null "None" "KeepRelative" "KeepRelative" "KeepRelative" true)
    (bind (_location _tangent) (`SplineComponent.GetLocationAndTangentAtSplinePoint` (`self.RailSpline`) _index "Local"))
    (bind (_location_2 _tangent_2) (`SplineComponent.GetLocationAndTangentAtSplinePoint` (`self.RailSpline`) (+ _index 1) "Local"))
    (`SplineMeshComponent.SetStartAndEnd` _returnvalue_2 _location _tangent _location_2 _tangent_2 true)
    (`StaticMeshComponent.SetStaticMesh` _returnvalue_2 (`self.RailMesh`))
    (`SplineMeshComponent.SetForwardAxis` _returnvalue_2 "Y" true)
    (`PrimitiveComponent.SetCollisionEnabled` _returnvalue_2 "QueryOnly")
    (`PrimitiveComponent.SetCollisionObjectType` _returnvalue_2 "ECC_GameTraceChannel2")
    (`KismetArrayLibrary.Array_AddUnique` (`self.RailMeshComponents`) _returnvalue_2))
  (if (not (`SplineComponent.IsClosedLoop` (`self.RailSpline`)))
    (bind _returnvalue_3 (`AddComponent|NODE_AddChildActorComponent-0`))
    (bind _asbp_homing_target_base (cast `/Game/LevelObjects/BP_HomingTarget_Base` (`ChildActorComponent.ChildActor` _returnvalue_3)))
    (set `self.StartHomingTarget` _asbp_homing_target_base)
    (`SceneComponent.K2_SetRelativeLocation` _returnvalue_3 (+ (+ (`SplineComponent.GetLocationAtSplinePoint` _railspline 0 "Local") (* (`SplineComponent.GetDirectionAtSplinePoint` _railspline 0 "Local") (`self.HomingTargetHorizontalOffset`))) (`KismetMathLibrary.MakeVector` 0.0 0.0 (`self.HomingTargetVerticalOffset`))) false false)
    (bind _returnvalue_4 (`AddComponent|NODE_AddChildActorComponent-1`))
    (bind _asbp_homing_target_base_2 (cast `/Game/LevelObjects/BP_HomingTarget_Base` (`ChildActorComponent.ChildActor` _returnvalue_4)))
    (set `self.EndHomingTarget` _asbp_homing_target_base_2)
    (`SceneComponent.K2_SetRelativeLocation` _returnvalue_4 (+ (+ (`SplineComponent.GetLocationAtSplinePoint` _railspline_2 _returnvalue "Local") (* (`SplineComponent.GetDirectionAtSplinePoint` _railspline_2 _returnvalue "Local") (* (`self.HomingTargetHorizontalOffset`) -1.0))) (`KismetMathLibrary.MakeVector` 0.0 0.0 (`self.HomingTargetVerticalOffset`))) false false)))