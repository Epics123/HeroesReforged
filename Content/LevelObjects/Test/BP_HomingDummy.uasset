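; BP_HomingDummy is a test level object that serves as a damageable target for Sonic's homing attack.
; When BP_Sonic overlaps its sphere, it applies Sonic's homing attack damage to its enemy health component and notifies Sonic of the hit, passing its homing target component.
; When health depletes, the bound event calls ForceDestroyWhenHit on the homing target component.
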(event `self.ReceiveBeginPlay`
  (add `EnemyHealthComponent.OnHealthDepleated` (`self.BPC_EnemyHealth`) (`|CreateDelegate` :!event `OnHealthDepleated`)))

(event `self.Sphere.OnComponentBeginOverlap`
  (params (OverlappedComponent :type "PrimitiveComponent Object Reference") (OtherActor :type "Actor Object Reference") (OtherComp :type "PrimitiveComponent Object Reference") (OtherBodyIndex :type Integer) (bFromSweep :type Boolean) (SweepResult :type "HitResult Structure (by ref)"))
  (bind _asbp_sonic (cast `/Game/Characters/Heroes/Sonic/BP_Sonic` OtherActor))
  (`EnemyHealthComponent.OnDamageTaken` (`self.BPC_EnemyHealth`) (`/Game/Characters/Heroes/Sonic/BP_Sonic.HomingAttackDamage` _asbp_sonic))
  (`/Game/Characters/Heroes/Sonic/BP_Sonic.HomingAttackHit` _asbp_sonic (`self.BPC_HomingTarget`)))

(event `OnHealthDepleated`
  (`/Game/Global/Components/BPC_HomingTarget.ForceDestroyWhenHit` (`self.BPC_HomingTarget`)))

(fn `UserConstructionScript`)