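; Sonic hero Blueprint that adds a homing attack and wall running to its parent character, with level-based attack stats.
; While falling, sphere traces pick the nearest in-view HomingTargetComponent; secondary jump homes in via timeline, or dashes forward without one.
; Side-on capsule hits start Flying-mode wall runs, steered along the traced wall tangent until speed or wall is lost.
; Jumping launches off walls; F is a level-up key.
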(event `self.OnLevelUp`
  (`parent.OnLevelUp`)
  (`self.UpdateHomingAttack`))

(event `self.ReceiveBeginPlay`
  (`parent.ReceiveBeginPlay`)
  (add `self.HomingAttackHit` (`|CreateDelegate` :!event `OnHomingAttackHit`)))

(event `self.ReceiveTick`
  (params (DeltaSeconds :type "Float (single-precision)"))
  (`parent.ReceiveTick` DeltaSeconds)
  (`self.TickWallRun` DeltaSeconds)
  (if (`NavMovementInterface.IsFalling` (`self.GetHeroMovementComponent`))
    (`self.FindHomingTargets`)))

(event `self.OnLevelReset`
  (`parent.OnLevelReset`)
  (`self.UpdateHomingAttack`))

(event `self.StartSecondaryJumpAction`
  (`parent.StartSecondaryJumpAction`)
  (`self.DoHomingAttack`))

(event `self.OnJumped`
  (`parent.OnJumped`)
  (`self.TryJumpOffWall`))

(event `self.OnLanded`
  (params (Hit :type "HitResult Structure (by ref)"))
  (`self.StopWallRun`)
  (`self.ResetHomingAttack`)
  (`parent.OnLanded` Hit))

(event `Key|F`
  (params (Key :type "Key Structure"))
  (:`Pressed`
    (`HeroLevelComponent.IncreaseLevel` (`self.LevelComponent`))
    (`KismetSystemLibrary.PrintString` (`KismetTextLibrary.Conv_TextToString` (`|FormatText` "Level Up! Current level: {Level}" (`self.GetHeroLevel`))))))

(event `DoHomingAttack`
  (bind _returnvalue (`self.GetHeroMovementComponent`))
  ;[0 0.4732 1 0.5] HomingAttack
  (if (and (`self.CanHomingAttack`) (not (`self.IsWallRunning`)))
    (`self.ShowJumpball`)
    (bind _returnvalue_2 (`NiagaraFunctionLibrary.SpawnSystemAttached` "/Game/Characters/Heroes/Sonic/FX/NS_HomingTrail.NS_HomingTrail" (`self.JumpballPivot`) "None" (0.0 0.0 0.0) (struct) "KeepRelativeOffset"))
    (set `self.HomingTrailFX` _returnvalue_2)
    (if (and (`KismetArrayLibrary.Array_IsNotEmpty` (`self.HomingTargets`)) (`KismetSystemLibrary.IsValid` (`self.CurrentHomingTarget`)))
      (set `self.IsInHomingAttack` true)
      (`MovementComponent.StopMovementImmediately` _returnvalue)
      (set `CharacterMovementComponent.GravityScale` 0.0 _returnvalue)
      (`self.MoveHomingAttack`)
      (else
        (`CharacterMovementComponent.AddImpulse` (`self.CharacterMovement`) (* (`self.GetActorForwardVector`) (`self.HomingAttackStrength`)) true)
        (set `self.CanHomingAttack` false)))))

(event `FindHomingTargets`
  ;[0 0.4732 1 0.5] HomingAttack
  (bind _targets (`self.GetHomingTargets`))
  (set `self.HomingTargets` _targets)
  (if (not (`self.IsInHomingAttack`))
    (bind _target (`self.GetBestHomingTarget`))
    (`self.HandleHomingTargetChanged` _target)))

(event `ResetHomingAttack`
  ;[0 0.4732 1 0.5] HomingAttack
  (bind _returnvalue (`KismetSystemLibrary.K2_SetTimerDelegate` (`|CreateDelegate` :!event `ResetCanHomingAttack`) (`self.HomingAttackCooldown`)))
  (set `self.CanHomingAttackTimer` _returnvalue)
  (`KismetArrayLibrary.Array_Clear` (`self.HomingTargets`))
  (`/Engine/EditorBlueprintResources/StandardMacros.IsValid` (`self.CurrentHomingTarget`)
    (:`Is Valid`
      (`HomingTargetComponent.HideHomingTarget` (`self.CurrentHomingTarget`)))
    (:`Is Not Valid`
      _))
  (set `self.CurrentHomingTarget` null)
  (`self.HideJumpball`)
  (`/Engine/EditorBlueprintResources/StandardMacros.IsValid` (`self.HomingTrailFX`)
    (:`Is Valid`
      (`SceneComponent.K2_DetachFromComponent` (`self.HomingTrailFX`) "KeepWorld" "KeepWorld" "KeepWorld" true))))

(event `OnHomingAttackHit` :!signature `self.HomingAttackHit`
  (params (HitTarget :type "HomingTargetComponent Object Reference"))
  ;[0 0.4732 1 0.5] HomingAttack
  (`HomingTargetComponent.HandleTargetHit` HitTarget self)
  (set `self.ShouldStopHomingAttack` true)
  (`self.HideJumpball`)
  (`NiagaraFunctionLibrary.SpawnSystemAttached` "/Game/Characters/Heroes/Sonic/FX/NS_HomingEnd.NS_HomingEnd" (`self.JumpballPivot`) "None" (0.0 0.0 0.0) (struct) "KeepRelativeOffset")
  (`self.PlayAnimMontage` "/Game/Characters/Heroes/Sonic/Anim/AM_Sonic_Homing_End.AM_Sonic_Homing_End"))

(event `MoveHomingAttack`
  ;[0 0.4732 1 0.5] HomingAttack
  (`Timeline|HomingTimeline` :!via `PlayFromStart`
    (:`Update`
      (`/Engine/EditorBlueprintResources/StandardMacros.IsValid` (`self.CurrentHomingTarget`)
        (:`Is Valid`
          (if (not (`self.ShouldStopHomingAttack`))
            (`self.K2_SetActorLocationAndRotation` (`KismetMathLibrary.VInterpTo` (`self.K2_GetActorLocation`) (`SceneComponent.K2_GetComponentLocation` (`self.CurrentHomingTarget`)) (`GameplayStatics.GetWorldDeltaSeconds`) (`self.HomingAttackSpeed`)) (`KismetMathLibrary.FindLookAtRotation` (`self.K2_GetActorLocation`) (`SceneComponent.K2_GetComponentLocation` (`self.CurrentHomingTarget`))))
            (else
              (`self.StopHomingAttack`))))
        (:`Is Not Valid`
          (`self.StopHomingAttack`))))
    (:`Finished`
      (`self.StopHomingAttack`))))

(event `ResetCanHomingAttack`
  ;[0 0.4732 1 0.5] HomingAttack
  (set `self.CanHomingAttack` true)
  (`KismetSystemLibrary.K2_ClearAndInvalidateTimerHandle` (`self.CanHomingAttackTimer`)))

(event `StopHomingAttack`
  (bind _homingtimeline (`self.HomingTimeline`))
  ;[0 0.4732 1 0.5] HomingAttack
  (set `self.IsInHomingAttack` false)
  (set `self.CanHomingAttack` false)
  (set `self.ShouldStopHomingAttack` false)
  (set `CharacterMovementComponent.GravityScale` 1.0 (`self.GetHeroMovementComponent`))
  (if (`TimelineComponent.IsPlaying` _homingtimeline)
    (`TimelineComponent.Stop` _homingtimeline))
  (`self.ResetHomingAttack`))

(event `self.CapsuleComponent.OnComponentHit`
  (params (HitComponent :type "PrimitiveComponent Object Reference") (OtherActor :type "Actor Object Reference") (OtherComp :type "PrimitiveComponent Object Reference") (NormalImpulse :type "Vector Structure") (Hit :type "HitResult Structure (by ref)"))
  (bind (_returnvalue _hitresult) (`self.ShouldAttachToWall` Hit 0.7))
  (if _returnvalue
    (`self.StartWallRun` (`.ImpactNormal` (`GameplayStatics.BreakHitResult` _hitresult)))
    (elif (`self.IsWallRunning`)
      (`self.StopWallRun`)
      (`CharacterMovementComponent.SetMovementMode` (`self.GetHeroMovementComponent`) "MOVE_Falling" 0))))

(event `UpdateWallRotation`
  (params (DeltaTime :type "Float (double-precision)"))
  (`self.K2_SetActorRotation` (`KismetMathLibrary.RInterpTo` (`self.K2_GetActorRotation`) (`KismetMathLibrary.MakeRotFromX` (`self.WallTangent`)) DeltaTime 15.0)))

(event `TryJumpOffWall`
  (bind _velocity (`MovementComponent.Velocity` (`self.GetHeroMovementComponent`)))
  (bind (_returnvalue_x _returnvalue_y) (`KismetMathLibrary.BreakVector` (* (+ (`self.CurrentWallNormal`) (`KismetMathLibrary.Normal` _velocity)) (`KismetMathLibrary.VSize` _velocity))))
  (if (`self.IsWallRunning`)
    (`self.StopWallRun`)
    (`CharacterMovementComponent.SetMovementMode` (`self.GetHeroMovementComponent`) "MOVE_Falling" 0)
    (`self.LaunchCharacter` (`KismetMathLibrary.MakeVector` _returnvalue_x _returnvalue_y 400.0) true)
    (`self.ResetCanHomingAttack`)))

(fn `GetBestHomingTarget`
  (returns (Target :type "HomingTargetComponent Object Reference"))
  (locals (ClosestTarget :type "HomingTargetComponent Object Reference") (ClosestDist :type "Float (double-precision)"))
  (set `local.ClosestDist` 10000.0)
  (for _array_element (`self.HomingTargets`)
    (bind _returnvalue (`KismetMathLibrary.Vector_Distance` (`self.K2_GetActorLocation`) (`SceneComponent.K2_GetComponentLocation` _array_element)))
    (if (and (< _returnvalue (`local.ClosestDist`)) (`self.IsHomingTargetInView` _array_element -0.65 0.65 -0.9 0.9))
      (set `local.ClosestTarget` _array_element)
      (set `local.ClosestDist` _returnvalue)))
  (return (`local.ClosestTarget`)))

(fn `GetHomingTargets`
  (returns (Targets :type "Array of HomingTargetComponent Object Reference"))
  (locals (FiundTargets :type "Array of HomingTargetComponent Object Reference"))
  (bind _returnvalue (`self.K2_GetActorLocation`))
  (bind _outhits (`KismetSystemLibrary.SphereTraceMultiForObjects` :`Start` _returnvalue :`End` _returnvalue :`Radius` (`self.HomingAttackRadius`) :`ObjectTypes` (`|MakeArray` "ObjectTypeQuery3" "ObjectTypeQuery2" :!type "EObjectTypeQuery Enum") :`DrawTime` 2.0))
  (for _array_element _outhits
    (bind _returnvalue_2 (`self.GetComponentByClass` (`.HitActor` (`GameplayStatics.BreakHitResult` _array_element)) "/Script/HeroesReforged.HomingTargetComponent"))
    (`/Engine/EditorBlueprintResources/StandardMacros.IsValid` _returnvalue_2
      (:`Is Valid`
        (`KismetArrayLibrary.Array_Add` (`local.FiundTargets`) _returnvalue_2))))
  (return (`local.FiundTargets`)))

(fn `HandleHomingTargetChanged`
  (params (NewTarget :type "HomingTargetComponent Object Reference"))
  (`/Engine/EditorBlueprintResources/StandardMacros.IsValid` (`self.CurrentHomingTarget`)
    (:`Is Valid`
      (if (not (== (`self.CurrentHomingTarget`) (`local.NewTarget`)))
        (`HomingTargetComponent.HideHomingTarget` (`self.CurrentHomingTarget`))
        (`/Engine/EditorBlueprintResources/StandardMacros.IsValid` (`local.NewTarget`) :!label _label
          (:`Is Valid`
            (bind _output_get (set `self.CurrentHomingTarget` (`local.NewTarget`)))
            (`HomingTargetComponent.ShowHomingTarget` _output_get)))))
    (:`Is Not Valid`
      (goto _label))))

(fn `IsHomingTargetInView`
  (params (Target :type "HomingTargetComponent Object Reference") (MinVerticalAngle :type "Float (double-precision)") (MaxVerticalAngle :type "Float (double-precision)") (MinHorizontalAngle :type "Float (double-precision)") (MaxHorizontalAngle :type "Float (double-precision)"))
  (returns (InView :type Boolean))
  (locals (DirToTarget :type "Vector Structure" :default (0.0 0.0 0.0)))
  (set `local.DirToTarget` (`KismetMathLibrary.Normal` (- (`SceneComponent.K2_GetComponentLocation` (`local.Target`)) (`self.K2_GetActorLocation`))))
  (return (and (>= (`KismetMathLibrary.Dot_VectorVector` (`KismetMathLibrary.GetForwardVector` (`self.GetControlRotation`)) (`local.DirToTarget`)) 0.0) (`KismetMathLibrary.InRange_FloatFloat` (`KismetMathLibrary.Dot_VectorVector` (`KismetMathLibrary.GetUpVector` (`self.GetControlRotation`)) (`local.DirToTarget`)) (`local.MinVerticalAngle`) (`local.MaxVerticalAngle`)) (`KismetMathLibrary.InRange_FloatFloat` (`KismetMathLibrary.Dot_VectorVector` (`KismetMathLibrary.GetRightVector` (`self.GetControlRotation`)) (`local.DirToTarget`)) (`local.MinHorizontalAngle`) (`local.MaxHorizontalAngle`)))))

(fn `ShouldAttachToWall`
  (params (Hit :type "HitResult Structure (by ref)") (AttachThreshold :type "Float (double-precision)"))
  (returns (ReturnValue :type Boolean) (HitResult :type "HitResult Structure (by ref)"))
  (return (> (`KismetMathLibrary.Abs` (`KismetMathLibrary.Dot_VectorVector` (`.Normal` (`GameplayStatics.BreakHitResult` Hit)) (`self.GetActorRightVector`))) (`local.AttachThreshold`)) Hit))

(fn `StartWallRun`
  (params (WallNormal :type "Vector Structure"))
  (bind _returnvalue (`self.GetHeroMovementComponent`))
  (bind _returnvalue_2 (> (`KismetMathLibrary.Dot_VectorVector` (`self.CurrentWallNormal`) (`self.GetActorRightVector`)) 0.0))
  (if (`NavMovementInterface.IsFalling` (`self.GetHeroMovementComponent`))
    (`self.ResetHomingAttack`)
    (set `self.CanHomingAttack` false)
    (set `self.IsWallRunning` true)
    (set `self.CurrentWallNormal` (`local.WallNormal`))
    (set `self.WallTangent` (`KismetMathLibrary.Cross_VectorVector` (`self.CurrentWallNormal`) (`KismetMathLibrary.SelectVector` (0.0 0.0 1.0) (0.0 0.0 -1.0) _returnvalue_2)))
    (set `self.WallRunDirection` (`KismetMathLibrary.SelectFloat` -1.0 1.0 _returnvalue_2))
    (`CharacterMovementComponent.SetMovementMode` _returnvalue "MOVE_Flying" 0)
    (set `CharacterMovementComponent.GravityScale` 0.0 _returnvalue)
    (set `HeroMovementComponent.bHasOverrideFallingRotation` true _returnvalue)
    (set `HeroMovementComponent.bForceCharacterVectors` true _returnvalue)
    (`SceneComponent.K2_SetRelativeLocation` (`self.Mesh`) (+ (* (`KismetMathLibrary.InverseTransformDirection` (`self.GetTransform`) (`self.CurrentWallNormal`)) (`self.WallRunMeshWallOffset`)) (`KismetMathLibrary.MakeVector` 0.0 0.0 (`self.WallRunMeshVerticalOffset`))) false false)))

(fn `StopWallRun`
  (bind _returnvalue (`self.GetHeroMovementComponent`))
  (`MovementComponent.SetPlaneConstraintEnabled` _returnvalue false)
  (set `CharacterMovementComponent.GravityScale` 1.0 _returnvalue)
  (set `self.IsWallRunning` false)
  (set `HeroMovementComponent.bHasOverrideFallingRotation` false _returnvalue)
  (set `HeroMovementComponent.bForceCharacterVectors` false _returnvalue)
  (`SceneComponent.K2_SetRelativeLocation` (`self.Mesh`) (0.0 0.0 -52.0) false false)
  (if (`|EnumEquality` (`CharacterMovementComponent.MovementMode` _returnvalue) "MOVE_Flying")
    (`CharacterMovementComponent.SetMovementMode` _returnvalue "MOVE_Falling" 0)))

(fn `TickWallRun`
  (params (DeltaTime :type "Float (double-precision)"))
  (locals (CurrentSpeed :type "Float (double-precision)" :default 0.0))
  (bind _returnvalue (`self.K2_GetActorLocation`))
  (bind _returnvalue_2 (`self.K2_GetActorLocation`))
  (bind _returnvalue_3 (`self.K2_GetActorLocation`))
  (bind (_returnvalue_x _returnvalue_y _returnvalue_z) (`KismetMathLibrary.BreakVector` (`self.GetLastMovementInputVector`)))
  (bind _returnvalue_4 (+ (`self.K2_GetActorLocation`) (* (`self.GetActorUpVector`) (* (`CapsuleComponent.CapsuleHalfHeight` (`self.CapsuleComponent`)) -1.0))))
  (set `local.CurrentSpeed` (`KismetMathLibrary.VSize` (`MovementComponent.Velocity` (`self.GetHeroMovementComponent`))))
  (if (and (`self.IsWallRunning`) (> (`KismetMathLibrary.Abs` (`local.CurrentSpeed`)) (`self.MinWallSpeed`)))
    (`self.UpdateWallRotation` (`local.DeltaTime`))
    (bind (_outhit _returnvalue_5) (`KismetSystemLibrary.SphereTraceSingle` _returnvalue_4 (+ _returnvalue_4 (* (`self.GetActorRightVector`) (`self.WallRunDirection`) 60.0)) 5.0 "TraceTypeQuery1"))
    (if _returnvalue_5
      (bind _output_get (set `self.CurrentWallNormal` (`.ImpactNormal` (`GameplayStatics.BreakHitResult` _outhit))))
      (`HeroMovementComponent.SetCurrentSurfaceNormal` (`self.GetHeroMovementComponent`) _output_get)
      (bind _output_get_2 (set `self.WallTangent` (`KismetMathLibrary.Cross_VectorVector` (`self.CurrentWallNormal`) (`KismetMathLibrary.SelectVector` (0.0 0.0 -1.0) (0.0 0.0 1.0) (> (`self.WallRunDirection`) 0.0)))))
      (set `MovementComponent.Velocity` (+ (* _output_get_2 (`local.CurrentSpeed`)) (`KismetMathLibrary.MakeVector` 0.0 0.0 (* _returnvalue_z (* (`local.CurrentSpeed`) (`CurveFloat.GetFloatValue` (`self.VerticalWallMultiplierCurve`) (`local.CurrentSpeed`)))))) (`self.GetHeroMovementComponent`))
      ; Debug Wall Run
      (bind _returnvalue_6 (`KismetSystemLibrary.GetConsoleVariableIntValue` "p.VisualizeMovement"))
      (if (!= _returnvalue_6 0)
        (`KismetSystemLibrary.DrawDebugArrow` _returnvalue_2 (+ _returnvalue_2 (* (`KismetMathLibrary.Normal` (`self.WallTangent`)) 50.0)) 0.0 (struct :`R` 0.969866 :`G` 0.007351 :`B` 1.0 :`A` 1.0))
        (`KismetSystemLibrary.DrawDebugArrow` _returnvalue_3 (+ _returnvalue_3 (* (`KismetMathLibrary.Normal` (`self.CurrentWallNormal`)) 50.0)) 0.0 (struct :`R` 1.0 :`G` 0.31318 :`A` 1.0))
        (`KismetSystemLibrary.DrawDebugArrow` _returnvalue (+ _returnvalue (* (`self.GetLastMovementInputVector`) 50.0)) 0.0 (struct :`R` 0.028789 :`G` 0.377327 :`B` 1.0 :`A` 1.0)))
      (else
        (`self.StopWallRun`)))
    (else
      (`self.StopWallRun`))))

(fn `UpdateHomingAttack`
  (set `self.HomingAttackDamage` (`|GetArrayItem` (`HomingAttackDefinition.DamageValues` (`self.HomingAttackDef`)) (`self.GetHeroLevel`)))
  (set `self.HomingAttackCooldown` (`|GetArrayItem` (`HomingAttackDefinition.CooldownTimes` (`self.HomingAttackDef`)) (`self.GetHeroLevel`))))

(fn `UserConstructionScript`
  (`parent.UserConstructionScript`))