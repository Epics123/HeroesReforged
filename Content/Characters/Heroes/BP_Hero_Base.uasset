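; Base hero character for Sonic-style movement, handling jumpball, rolling and rail grinding, with stub events for child classes.
; Capsule hits on rails trigger attachment, switching to Flying movement with grind speed and sparks; detaching restores values and drops to Falling.
; Rail switches detach, then a timeline interpolates the hero toward the closest point on the target spline.
; Crouching caches slope, acceleration and friction, applies roll values when rolling, and restores them on uncrouch.
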(event `self.ReceiveBeginPlay`
  (`parent.ReceiveBeginPlay`)
  (add `self.OnReachedJumpApex` (`|CreateDelegate` :!event `OnApexReached`))
  (bind _returnvalue (`NiagaraFunctionLibrary.SpawnSystemAttached` "/Game/Characters/Heroes/Sonic/FX/NS_RailGrind_Metal.NS_RailGrind_Metal" (`self.Mesh`) "GrindFXPoint_R" (0.0 0.0 0.0) (struct) "SnapToTarget"))
  (set `self.RailFX_R` _returnvalue)
  (bind _returnvalue_2 (`NiagaraFunctionLibrary.SpawnSystemAttached` "/Game/Characters/Heroes/Sonic/FX/NS_RailGrind_Metal.NS_RailGrind_Metal" (`self.Mesh`) "GrindFXPoint_L" (0.0 0.0 0.0) (struct) "SnapToTarget"))
  (set `self.RailFX_L` _returnvalue_2)
  (`self.ToggleRailVFX` true))

(event `self.OnJumped`
  (`parent.OnJumped`)
  (if (`self.bOnRail`)
    (`self.TryDetachFromRail`)
    (`self.PlayAnimMontage` "/Game/Characters/Heroes/Sonic/Anim/AM_Sonic_Grind_Jump.AM_Sonic_Grind_Jump")
    (else
      (`self.ShowJumpball`)
      (set `HeroMovementComponent.bSkipRotateToVelocity` true (`self.GetHeroMovementComponent`)))))

(event `OnApexReached`)

(event `self.OnLanded`
  (params (Hit :type "HitResult Structure (by ref)"))
  (bind _returnvalue (`self.GetHeroMovementComponent`))
  (`parent.OnLanded` Hit)
  (set `HeroMovementComponent.bSkipRotateToVelocity` false _returnvalue)
  (set `CharacterMovementComponent.bOrientRotationToMovement` false _returnvalue)
  (set `self.FallFromRail` false)
  (`self.CancelRailSwitch`))

(event `self.ReceiveTick`
  (params (DeltaSeconds :type "Float (single-precision)")))

(event `self.OnSwapRail`
  (params (Direction :type "Float (single-precision)"))
  (`/Engine/EditorBlueprintResources/StandardMacros.IsValid` (`self.CurrentRail`)
    (:`Is Valid`
      (`/Engine/EditorBlueprintResources/StandardMacros.IsValid` (`self.JumpRail`)
        (:`Is Valid`
          (if (== (`KismetMathLibrary.Round` Direction) (`KismetMathLibrary.Round` (`self.RailLeanDirection`)))
            (`self.PlayAnimMontage` (select `bool` (> (`KismetMathLibrary.Round` Direction) 0) :`false` "/Game/Characters/Heroes/Sonic/Anim/AM_Sonic_GrindJump_L.AM_Sonic_GrindJump_L" :`true` "/Game/Characters/Heroes/Sonic/Anim/AM_Sonic_GrindJump_R.AM_Sonic_GrindJump_R" :!type "AnimMontage Object Reference"))))))))

(event `DoRailSwitch`
  (bind _returnvalue (`self.K2_GetActorLocation`))
  (`self.TryDetachFromRail`)
  (`Timeline|Timeline` :!via `PlayFromStart` :!label _label
    (:`Update`
      (`/Engine/EditorBlueprintResources/StandardMacros.IsValid` (`self.JumpRail`)
        (:`Is Valid`
          (`self.K2_SetActorLocation` (`KismetMathLibrary.VInterpTo` (`self.K2_GetActorLocation`) (+ (`SplineComponent.FindLocationClosestToWorldLocation` (`RailBase.RailSpline` (`self.JumpRail`)) _returnvalue "World") (* (`SplineComponent.FindUpVectorClosestToWorldLocation` (`RailBase.RailSpline` (`self.JumpRail`)) _returnvalue "World") (`RailBase.RailVerticalOffset` (`self.JumpRail`)))) (`GameplayStatics.GetWorldDeltaSeconds`) 7.0)))))))

(event `CancelRailSwitch`
  (`self.ToggleRailVFX` true)
  (goto _label :!via `Stop`))

(event `self.OnLevelUp`)

(event `self.OnLevelReset`)

(event `OnHomingAttackHit`
  (params (HitTarget :type "HomingTargetComponent Object Reference")))

(event `self.CapsuleComponent.OnComponentHit`
  (params (HitComponent :type "PrimitiveComponent Object Reference") (OtherActor :type "Actor Object Reference") (OtherComp :type "PrimitiveComponent Object Reference") (NormalImpulse :type "Vector Structure") (Hit :type "HitResult Structure (by ref)"))
  (bind _asbp_rail_base (cast `/Game/LevelObjects/Rails/BP_RailBase` OtherActor))
  (if (not (`self.bOnRail`))
    (`RailBase.SetRailActiveState` _asbp_rail_base true)
    (`self.TryAttachToRail` _asbp_rail_base)))

(event `self.OnRailEnd`
  (params (Rail :type "RailBase Object Reference"))
  (`self.CancelRailSwitch`)
  (`self.TryDetachFromRail`))

(event `self.K2_OnStartCrouch`
  (params (HalfHeightAdjust :type "Float (single-precision)") (ScaledHalfHeightAdjust :type "Float (single-precision)"))
  (`parent.K2_OnStartCrouch` HalfHeightAdjust ScaledHalfHeightAdjust)
  (`self.CachePreRollMovement`)
  (if (`self.bRolling`)
    (`self.ApplyRollMovement`)))

(event `self.K2_OnEndCrouch`
  (params (HalfHeightAdjust :type "Float (single-precision)") (ScaledHalfHeightAdjust :type "Float (single-precision)"))
  (`parent.K2_OnEndCrouch` HalfHeightAdjust ScaledHalfHeightAdjust)
  (`self.ResetRollMovement`))

(event `ApplyRollMovement`
  (bind _returnvalue (`self.GetHeroMovementComponent`))
  (set `HeroMovementComponent.SlopeEffectThreshold` (`self.RollSlopeThreshold`) _returnvalue)
  (set `CharacterMovementComponent.MaxAcceleration` (`self.RollAcceleration`) _returnvalue)
  (set `CharacterMovementComponent.GroundFriction` (`self.RollFriction`) _returnvalue))

(event `ResetRollMovement`
  (bind _returnvalue (`self.GetHeroMovementComponent`))
  (set `HeroMovementComponent.SlopeEffectThreshold` (`self.PreRollSlopeThreshold`) _returnvalue)
  (set `CharacterMovementComponent.MaxAcceleration` (`self.PreRollAcceleration`) _returnvalue)
  (set `CharacterMovementComponent.GroundFriction` (`self.PreRollGroundFriction`) _returnvalue))

(event `CachePreRollMovement`
  (bind _returnvalue (`self.GetHeroMovementComponent`))
  (set `self.PreRollSlopeThreshold` (`HeroMovementComponent.SlopeEffectThreshold` _returnvalue))
  (set `self.PreRollAcceleration` (`CharacterMovementComponent.GetMaxAcceleration` _returnvalue))
  (set `self.PreRollGroundFriction` (`CharacterMovementComponent.GroundFriction` _returnvalue)))

(fn `ToggleRailVFX`
  (params (Hidden :type Boolean))
  ; TODO: Pick rail vfx based on rail type
  (`NiagaraComponent.SetPaused` (`self.RailFX_R`) (`local.Hidden`))
  (`NiagaraComponent.SetPaused` (`self.RailFX_L`) (`local.Hidden`))
  (`SceneComponent.SetHiddenInGame` (`self.RailFX_R`) (`local.Hidden`) false)
  (`SceneComponent.SetHiddenInGame` (`self.RailFX_L`) (`local.Hidden`) false))

(fn `TryAttachToRail`
  (params (Rail :type "/Game/LevelObjects/Rails/BP_RailBase Object Reference"))
  (bind _returnvalue (`self.GetHeroMovementComponent`))
  (bind _returnvalue_2 (`RailBase.AttachToRail` (`local.Rail`)))
  (if _returnvalue_2
    (set `self.bForceStopRoll` true)
    (`self.UnCrouch`)
    (`self.ResetRollMovement`)
    (`self.HideJumpball`)
    (set `self.bCanSpindash` false)
    (`CharacterMovementComponent.SetMovementMode` _returnvalue "MOVE_Flying" 0)
    (set `HeroMovementComponent.bForceCharacterVectors` true _returnvalue)
    (set `HeroMovementComponent.bSkipRotateToVelocity` false _returnvalue)
    (set `CharacterMovementComponent.bOrientRotationToMovement` false _returnvalue)
    (set `self.CachedBraking Deceleration Flying` (`CharacterMovementComponent.BrakingDecelerationFlying` _returnvalue))
    (set `CharacterMovementComponent.BrakingDecelerationFlying` 0.0 _returnvalue)
    (set `CharacterMovementComponent.MaxFlySpeed` (`HeroMovementComponent.MaxSpeedGrinding` _returnvalue) _returnvalue)
    (set `self.CachedMaxAcceleration` (`CharacterMovementComponent.MaxAcceleration` _returnvalue))
    (set `CharacterMovementComponent.MaxAcceleration` (`HeroMovementComponent.RailGrindingAcceleration` _returnvalue) _returnvalue)
    (set `self.FallFromRail` false)
    (`self.ToggleRailVFX` false)))

(fn `TryDetachFromRail`
  (bind _returnvalue (`self.GetHeroMovementComponent`))
  (`/Engine/EditorBlueprintResources/StandardMacros.IsValid` (`self.CurrentRail`)
    (:`Is Valid`
      (`RailBase.SetRailActiveState` (`self.CurrentRail`) false)
      (`RailBase.DetachFromRail` (`self.CurrentRail`))
      (`CharacterMovementComponent.SetMovementMode` _returnvalue "MOVE_Falling" 0)
      (set `HeroMovementComponent.bForceCharacterVectors` false _returnvalue)
      (set `CharacterMovementComponent.BrakingDecelerationFlying` (`self.CachedBraking Deceleration Flying`) _returnvalue)
      (set `CharacterMovementComponent.MaxFlySpeed` (`CharacterMovementComponent.MaxWalkSpeed` _returnvalue) _returnvalue)
      (set `CharacterMovementComponent.MaxAcceleration` (`self.CachedMaxAcceleration`) _returnvalue)
      (set `self.FallFromRail` true)
      (`self.ToggleRailVFX` true)
      (set `self.bCanSpindash` true))
    (:`Is Not Valid`
      (`self.ToggleRailVFX` true)
      (set `self.bCanSpindash` true))))

(fn `UserConstructionScript`)