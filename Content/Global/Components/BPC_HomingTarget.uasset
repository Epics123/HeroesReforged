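; BPC_HomingTarget is a component that gives a homing target an on-screen icon.
; On BeginPlay it creates a WB_HomingIcon widget at its world location with zero offset and adds it to the viewport, then removes it on EndPlay.
; ShowHomingTarget and HideHomingTarget forward to the widget to toggle the icon, and showing is skipped while the component is being destroyed.
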(event `self.ReceiveBeginPlay`
  (`self.CreateHomingIconWidget` (0.0 0.0 0.0) (`self.K2_GetComponentLocation`)))

(event `self.ReceiveEndPlay`
  (params (EndPlayReason :type "EEndPlayReason Enum" :default "Destroyed"))
  (`self.DestroyHomingIconWidget`))

(event `self.ShowHomingTarget`
  (`/Engine/EditorBlueprintResources/StandardMacros.IsValid` (`self.HomingIconWidget`)
    (:`Is Valid`
      (if (not (`self.IsBeingDestroyed`))
        (`/Game/UI/Icons/HomingAttack/WB_HomingIcon.ShowHomingIcon` (`self.HomingIconWidget`))))))

(event `self.HideHomingTarget`
  (`/Engine/EditorBlueprintResources/StandardMacros.IsValid` (`self.HomingIconWidget`)
    (:`Is Valid`
      (`/Game/UI/Icons/HomingAttack/WB_HomingIcon.HideHomingIcon` (`self.HomingIconWidget`)))))

(event `CreateHomingIconWidget`
  (params (Offset :type "Vector Structure") (TargetLocation :type "Vector Structure"))
  (bind _returnvalue (`|CreateWidget` "/Game/UI/Icons/HomingAttack/WB_HomingIcon.WB_HomingIcon_C" null Offset TargetLocation))
  (bind _output_get (set `self.HomingIconWidget` _returnvalue))
  (`UserWidget.AddToViewport` _output_get 0))

(event `DestroyHomingIconWidget`
  (`/Engine/EditorBlueprintResources/StandardMacros.IsValid` (`self.HomingIconWidget`)
    (:`Is Valid`
      (`Widget.RemoveFromParent` (`self.HomingIconWidget`)))))